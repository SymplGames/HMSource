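; BP_TileManager spawns a chain of track tiles and builds the movement spline that a registered pawn receives.
; RegisterPawn takes the pawn's theme and lays the start tiles, and SpawnNextTile appends further tiles at the last tile's next transform.
; Each spawn runs a navmesh pathfind from the spline's end to the new tile's nav point, adding the path points to the spline.
; It tracks live tiles, removing them when destroyed.
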(event `self.ReceiveBeginPlay`
  (`parent.ReceiveBeginPlay`)
  (bind _outactors (`GameplayStatics.GetAllActorsOfClass` "/Script/NavigationSystem.NavMeshBoundsVolume"))
  (set `self.NavMesh` (`|GetArrayItem` _outactors)))

(fn `CleanTiles`
  (if (> (`KismetArrayLibrary.Array_Length` (`self.Tiles`)) 0)
    (`self.SetLifeSpan` (`self.Tiles`) 0.1)
    (`KismetArrayLibrary.Array_Clear` (`self.Tiles`))
    (set `self.LastTile` null)))

(fn `GetLastTile`
  (returns (LastTile :type "/Game/_Sympl/HyperlaneMessenger/Core/BP_Tile Object Reference"))
  (return (`self.LastTile`)))

(fn `GetTileCount`
  (returns (TileCount :type Integer))
  (return (`self.TileCount`)))

(fn `GetTiles`
  (returns (Tiles :type "Array of /Game/_Sympl/HyperlaneMessenger/Core/BP_Tile Object Reference"))
  (return (`self.Tiles`)))

(fn `RegisterPawn`
  (params (Pawn :type "/Game/_Sympl/HyperlaneMessenger/Core/Player/HyperlaneMessengerPawn Object Reference"))
  (`/Game/_Sympl/HyperlaneMessenger/Core/Player/HyperlaneMessengerPawn.Server_SetSplinePoint` Pawn (`self.MovementSpline`) self)
  (set `self.Themes` (`|MakeArray` (`/Game/_Sympl/HyperlaneMessenger/Core/Player/HyperlaneMessengerPawn.GetTileTheme` (`local.Pawn`))))
  (`self.SpawnStartTiles`))

(fn `RegisterTile`
  (params (Tile :type "Actor Object Reference"))
  (add `self.OnDestroyed` (`local.Tile`) (`|CreateDelegate` :!event `TileDestroyed`))
  (bind _asbp_tile (cast `/Game/_Sympl/HyperlaneMessenger/Core/BP_Tile` (`local.Tile`)))
  (`KismetArrayLibrary.Array_Add` (`self.Tiles`) _asbp_tile)
  (`/Engine/EditorBlueprintResources/StandardMacros.IncrementInt` (`self.TileCount`)))

(fn `SpawnNextTile`
  (params (Class :type "/Game/_Sympl/HyperlaneMessenger/Core/BP_Tile Class Reference"))
  (returns (LastTile :type "/Game/_Sympl/HyperlaneMessenger/Core/BP_Tile Object Reference"))
  (bind _lasttile (`self.SpawnTile` Class (`/Game/_Sympl/HyperlaneMessenger/Core/BP_Tile.GetNextTileTransform` (`self.GetLastTile`))))
  (return _lasttile))

(fn `SpawnStartTiles`
  (`self.CleanTiles`)
  (`self.SpawnTile` (`self.StartTileClass`) (`KismetMathLibrary.MakeTransform` (0.0 0.0 0.0)) false)
  (for _ (range 1 (`self.StartTiles`))
    (`self.SpawnTile` (`self.StartTileClass`) (`/Game/_Sympl/HyperlaneMessenger/Core/BP_Tile.GetNextTileTransform` (`self.LastTile`)) false)))

(fn `SpawnTile`
  (params (Class :type "/Game/_Sympl/HyperlaneMessenger/Core/BP_Tile Class Reference") (SpawnTransform :type "Transform Structure") (bCanSpawn :type Boolean :default true))
  (returns (LastTile :type "/Game/_Sympl/HyperlaneMessenger/Core/BP_Tile Object Reference"))
  (bind _movementspline (`self.MovementSpline`))
  (bind _returnvalue (`|SpawnActorFromClass` (`local.Class`) (`local.SpawnTransform`) "AlwaysSpawn" "OverrideRootScale" (`GameplayStatics.GetPlayerController` 0) (`self.Themes`) self (`self.bMatchThemeForAllTilePrimitives`) (`local.bCanSpawn`) (`self.TileCount`) (`self.SelectedThemeIndex`) (`GameplayStatics.GetPlayerPawn` 0)))
  (`self.RegisterTile` _returnvalue)
  (set `self.LastTile` _returnvalue)
  (bind _navmesh (`self.NavMesh`)
    (:`then`
      (bind _returnvalue_2 (`NavigationSystemV1.FindPathToLocationSynchronously` (`SplineComponent.GetLocationAtSplinePoint` _movementspline (- (`SplineComponent.GetNumberOfSplinePoints` _movementspline) 1) "World") (`/Game/_Sympl/HyperlaneMessenger/Core/BP_Tile.GetNavPoint` (`self.GetLastTile`)) _navmesh null))
      (for _array_element (`NavigationPath.PathPoints` _returnvalue_2)
        (`SplineComponent.AddSplinePoint` (`self.MovementSpline`) _array_element "World" true))
      (return (`self.GetLastTile`)))
    (:`else`
      (return (`self.GetLastTile`)))))

(fn `TileDestroyed`
  (params (DestroyedActor :type "Actor Object Reference"))
  (bind _asbp_tile (cast `/Game/_Sympl/HyperlaneMessenger/Core/BP_Tile` DestroyedActor))
  (`KismetArrayLibrary.Array_RemoveItem` (`self.Tiles`) _asbp_tile))

(fn `UserConstructionScript`)