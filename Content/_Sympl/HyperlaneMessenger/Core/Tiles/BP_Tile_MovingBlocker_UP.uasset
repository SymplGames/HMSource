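; Hyperlane Messenger tile with a blocker that moves back and forth, the upward-moving variant of the other tiles.
; Tick offsets WallF1 by OffsetDirection, reversing it and toggling Flip when the BlockerAtEnd or BlockerAtStart check passes.
; The construction script randomly picks one of two rotations for WallF1.
; An overlap on WallL1 calls GameOverHit with the other actor.
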(event `self.ReceiveTick`
  (params (DeltaSeconds :type "Float (single-precision)"))
  (`parent.ReceiveTick` DeltaSeconds)
  ;[0 0 0] Same as the other tiles, but this one moves up!
  (`SceneComponent.K2_AddLocalOffset` (`self.WallF1`) (`self.OffsetDirection`) false false)
  (if (select `bool` (`self.bFlip`) :`false` (`self.BlockerAtEnd`) :`true` (`self.BlockerAtStart`))
    (set `self.OffsetDirection` (* (`self.OffsetDirection`) -1))
    (set `self.bFlip` (not (`self.bFlip`)))))

(event `self.WallL1.OnComponentBeginOverlap`
  (params (OverlappedComponent :type "PrimitiveComponent Object Reference") (OtherActor :type "Actor Object Reference") (OtherComp :type "PrimitiveComponent Object Reference") (OtherBodyIndex :type Integer) (bFromSweep :type Boolean) (SweepResult :type "HitResult Structure (by ref)"))
  ;[0 0 0] Game over hit on overlap blocker
  (`self.GameOverHit` OtherActor))

(fn `UserConstructionScript`
  (`parent.UserConstructionScript`)
  (`SceneComponent.K2_SetRelativeRotation` (`self.WallF1`) (`KismetMathLibrary.SelectRotator` (struct :`Yaw` 90.0) (struct) (`KismetMathLibrary.RandomBool`)) false false))