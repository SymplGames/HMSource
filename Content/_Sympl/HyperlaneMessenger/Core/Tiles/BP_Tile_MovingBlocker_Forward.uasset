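; Moving-blocker tile for Hyperlane Messenger, a forward variant that duplicates the move-right tile's logic in a separate class.
; Each tick it offsets WallF1 by OffsetDirection, reversing on reaching the Arrow or FlipPoint location within a small tolerance, with a Flip flag selecting the target.
; A HyperlaneMessengerPawn overlapping WallL1, rather than the moving WallF1, triggers that pawn's GameOver.
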(event `self.ReceiveTick`
  (params (DeltaSeconds :type "Float (single-precision)"))
  (bind _wallf1 (`self.WallF1`))
  (bind _returnvalue (`SceneComponent.K2_GetComponentLocation` _wallf1))
  ;[1 1 1] Same as the move right tile. When I made it, I didn't realize that I didn't need a separate class, but it functions the same way. I didn't want to delete it, but you can delete this class and create a new subclass with different arrow points to avoid making multiple changes across classes if you want to update the way this works.
  (`parent.ReceiveTick` DeltaSeconds)
  (`SceneComponent.K2_AddLocalOffset` _wallf1 (`self.OffsetDirection`) false false)
  (if (select `bool` (`self.bFlip`) :`false` (== (`SceneComponent.K2_GetComponentLocation` (`self.FlipPoint`)) _returnvalue :`ErrorTolerance` 1.0) :`true` (== (`SceneComponent.K2_GetComponentLocation` (`self.Arrow`)) _returnvalue :`ErrorTolerance` 1.0))
    (set `self.OffsetDirection` (* (`self.OffsetDirection`) -1))
    (set `self.bFlip` (not (`self.bFlip`)))))

(event `self.WallL1.OnComponentBeginOverlap`
  (params (OverlappedComponent :type "PrimitiveComponent Object Reference") (OtherActor :type "Actor Object Reference") (OtherComp :type "PrimitiveComponent Object Reference") (OtherBodyIndex :type Integer) (bFromSweep :type Boolean) (SweepResult :type "HitResult Structure (by ref)"))
  ;[1 1 1] Same as the move right tile. When I made it, I didn't realize that I didn't need a separate class, but it functions the same way. I didn't want to delete it, but you can delete this class and create a new subclass with different arrow points to avoid making multiple changes across classes if you want to update the way this works.
  (bind _ashyperlane_messenger_pawn (cast `/Game/_Sympl/HyperlaneMessenger/Core/Player/HyperlaneMessengerPawn` OtherActor))
  (`/Game/_Sympl/HyperlaneMessenger/Core/Player/HyperlaneMessengerPawn.GameOver` _ashyperlane_messenger_pawn))

(fn `UserConstructionScript`
  (`parent.UserConstructionScript`))