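; Hyperlane Messenger tile with a blocker that shuttles between two movable arrow points and ends the game when the player pawn overlaps it.
; Each tick offsets WallL1 locally by OffsetDirection, without sweeping, then reverses it and toggles Flip when ShouldFlip returns true.
; ShouldFlip holds a tolerance check of the wall against Arrow or FlipPoint, chosen by Flip, but that check appears unconnected.
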(event `self.ReceiveTick`
  (params (DeltaSeconds :type "Float (single-precision)"))
  ;[1 1 1] A fun tile to move a blocker that kills the player. The blocker filps if the location matches the start or end arrow. You can move the arrows to any point you'd like and it should work!
  (`parent.ReceiveTick` DeltaSeconds)
  (`SceneComponent.K2_AddLocalOffset` (`self.WallL1`) (`self.OffsetDirection`) false false)
  (if (`self.ShouldFlip`)
    (set `self.OffsetDirection` (* (`self.OffsetDirection`) -1))
    (set `self.bFlip` (not (`self.bFlip`)))))

(event `self.WallL1.OnComponentBeginOverlap`
  (params (OverlappedComponent :type "PrimitiveComponent Object Reference") (OtherActor :type "Actor Object Reference") (OtherComp :type "PrimitiveComponent Object Reference") (OtherBodyIndex :type Integer) (bFromSweep :type Boolean) (SweepResult :type "HitResult Structure (by ref)"))
  ;[1 1 1] A fun tile to move a blocker that kills the player. The blocker filps if the location matches the start or end arrow. You can move the arrows to any point you'd like and it should work!
  (bind _ashyperlane_messenger_pawn (cast `/Game/_Sympl/HyperlaneMessenger/Core/Player/HyperlaneMessengerPawn` OtherActor))
  (`/Game/_Sympl/HyperlaneMessenger/Core/Player/HyperlaneMessengerPawn.GameOver` _ashyperlane_messenger_pawn))

(fn `UserConstructionScript`
  (`parent.UserConstructionScript`))